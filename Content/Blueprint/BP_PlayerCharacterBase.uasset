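; Base player character that turns input into movement, jumping, mouse look, weapon fire and ability use.
; Mouse X drives controller yaw, while mouse Y accumulates a clamped pitch applied directly to the View component.
; AbilityHolder supplies the weapon and abilities: fire requires an equipped weapon, though primary fire always calls CallFireEventDispatcher first.
; Ability 1 is gated by its cooldown, while the Ability 2 and 3 functions are empty stubs.
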(event `InputAction|Ability1`
  (params (Key :type "Key Structure"))
  (:`Pressed`
    (`self.UseAbility1`)))

(event `InputAction|Ability2`
  (params (Key :type "Key Structure"))
  (:`Pressed`
    (`self.UseAbility2`)))

(event `InputAction|Ability3`
  (params (Key :type "Key Structure"))
  (:`Pressed`
    (`self.UseAbility3`)))

(event `InputAction|PrimaryFire` :consume false
  (params (Key :type "Key Structure"))
  (:`Pressed`
    (`self.Fire Event Dispatcher`)
    (if (`/Game/Blueprint/BP_WeaponBase.Equipped` (`/Game/Blueprint/BP_AbilityHolder.Weapon` (`self.AbilityHolder`)))
      (`/Game/Blueprint/BP_WeaponBase.Do Primary Fire` (`/Game/Blueprint/BP_AbilityHolder.Weapon` (`self.AbilityHolder`))))))

(event `InputAction|SecondaryFire`
  (params (Key :type "Key Structure"))
  (:`Pressed`
    (if (`/Game/Blueprint/BP_WeaponBase.Equipped` (`/Game/Blueprint/BP_AbilityHolder.Weapon` (`self.AbilityHolder`)))
      (`/Game/Blueprint/BP_WeaponBase.Do Secondary Fire` (`/Game/Blueprint/BP_AbilityHolder.Weapon` (`self.AbilityHolder`))))))

(event `InputAction|Jump`
  (params (Key :type "Key Structure"))
  (:`Pressed`
    (`self.Jump`)))

(event `InputAxisKey|MouseX`
  (params (AxisValue :type "Float (single-precision)"))
  (`self.AddControllerYawInput` AxisValue))

(event `InputAxisKey|MouseY`
  (params (AxisValue :type "Float (single-precision)"))
  (bind _output_get (set `self.ViewRotation` (`KismetMathLibrary.FClamp` (+ AxisValue (`self.ViewRotation`)) -90.0 90.0)))
  (`SceneComponent.K2_SetRelativeRotation` (`self.View`) (`KismetMathLibrary.MakeRotator` 0.0 _output_get) false false))

(event `InputAxis|ForwardMovement`
  (params (AxisValue :type "Float (single-precision)"))
  (`self.AddMovementInput` (* (`SceneComponent.GetForwardVector` (`self.CapsuleComponent`)) AxisValue)))

(event `InputAxis|RightMovement`
  (params (AxisValue :type "Float (single-precision)"))
  (`self.AddMovementInput` (* (`SceneComponent.GetRightVector` (`self.CapsuleComponent`)) AxisValue)))

(fn `UseAbility1`
  (bind _ability1 (`/Game/Blueprint/BP_AbilityHolder.Ability1` (`self.AbilityHolder`)))
  (if (<= (`/Game/Blueprint/BP_AbilityBase.CurrentCooldownTime` _ability1) 0.0)
    (`/Game/Blueprint/BP_AbilityBase.Use Ability` _ability1)))

(fn `UseAbility2`)

(fn `UseAbility3`)

(fn `UserConstructionScript`)