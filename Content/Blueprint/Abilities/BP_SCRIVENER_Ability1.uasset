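; First ability of the Scrivener character: a toggled targeting mode that previews its placement with a decal.
; Using it swaps out the weapon and spawns the decal; using it again removes the decal and re-equips the weapon.
; While equipped, Tick line-traces from the player's view and projects the decal along the hit surface normal.
; The player's fire dispatcher triggers the parent ability and clears Equipped, leaving decal and weapon untouched here.
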(event `self.ReceiveBeginPlay`
  (`parent.ReceiveBeginPlay`)
  (bind _asbp_player_character_base (cast `/Game/Blueprint/BP_PlayerCharacterBase` (`self.GetOwner`)))
  (set `self.Player` _asbp_player_character_base)
  (add `/Game/Blueprint/BP_PlayerCharacterBase.Fire Event Dispatcher` (`self.Player`) (delegate `Fire`)))

(event `self.Use Ability`
  (if (`self.Equipped`)
    (set `self.Equipped` false)
    (`self.K2_DestroyComponent` (`self.CurrentDecal`))
    (set `self.CurrentDecal` null)
    (`/Game/Blueprint/BP_WeaponBase.Equip` (`/Game/Blueprint/BP_AbilityHolder.Weapon` (`/Game/Blueprint/BP_PlayerCharacterBase.AbilityHolder` (`self.Player`))))
    (else
      (`/Game/Blueprint/BP_WeaponBase.Unequip` (`/Game/Blueprint/BP_AbilityHolder.Weapon` (`/Game/Blueprint/BP_PlayerCharacterBase.AbilityHolder` (`self.Player`))))
      (set `self.Equipped` true)
      (bind _returnvalue (`GameplayStatics.SpawnDecalAtLocation` "/Game/DecalMaterial/MAT_SCRIVENERAbility1Decal.MAT_SCRIVENERAbility1Decal" (`KismetMathLibrary.Conv_DoubleToVector` (`self.DecalSize`))))
      (set `self.CurrentDecal` _returnvalue))))

(event `Fire`
  (`KismetSystemLibrary.PrintString` "Hello")
  (if (`self.Equipped`)
    (`parent.Use Ability`)
    (set `self.Equipped` false)))

(event `self.ReceiveTick`
  (params (DeltaSeconds :type "Float (single-precision)"))
  (bind _currentdecal (`self.CurrentDecal`))
  (`parent.ReceiveTick` DeltaSeconds)
  (if (`self.Equipped`)
    (bind _asbp_player_character_base (cast `/Game/Blueprint/BP_PlayerCharacterBase` (`self.GetOwner`)))
    (bind _view (`/Game/Blueprint/BP_PlayerCharacterBase.View` _asbp_player_character_base))
    (bind _returnvalue (`SceneComponent.K2_GetComponentLocation` _view))
    (bind (_outhit _returnvalue_2) (`KismetSystemLibrary.LineTraceSingle` _returnvalue (+ _returnvalue (* (`SceneComponent.GetForwardVector` _view) (`self.MaxDistance`))) "TraceTypeQuery1" true))
    (if _returnvalue_2
      (bind (_bblockinghit _binitialoverlap _time _distance _location _impactpoint _normal _impactnormal) (`GameplayStatics.BreakHitResult` _outhit))
      (bind _returnvalue_3 (+ _impactpoint (* _impactnormal (- (`self.DecalSize`) 5.0))))
      (`SceneComponent.K2_SetWorldLocation` _currentdecal _returnvalue_3 false false)
      (`SceneComponent.K2_SetWorldRotation` _currentdecal (`KismetMathLibrary.FindLookAtRotation` _returnvalue_3 (+ _returnvalue_3 (* _impactnormal -1.0))) false false))))